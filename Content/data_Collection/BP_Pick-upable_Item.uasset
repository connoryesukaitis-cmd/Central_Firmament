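; BP_Pick-upable_Item is a collectible data item that increments the first-person character's DataCount when picked up.
; A sphere overlap shows a widget while the character is in range if CanInteract is set, and hides it on exit, also clearing CanRessE.
; The Pick-upItems event, with no caller in this graph, adds to the count, plays a 2D sound and destroys the actor.
; A separate CustomEvent only branches on CanInteract, with no effect.
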(event OnComponentBeginOverlap(Sphere)
  (params (OverlappedComponent :type Primitive%20Component%20Object%20Reference) (OtherActor :type Actor%20Object%20Reference) (OtherComp :type Primitive%20Component%20Object%20Reference) (OtherBodyIndex :type Integer) (bFromSweep :type Boolean) (SweepResult :type Hit%20Result%20Structure%20%28by%20ref%29))
  (Utilities|Casting|CastToBP_FirstPersonCharacter OtherActor)
  (if (Variables|Default|GetCanInteract)
    (Rendering|SetVisibility (Variables|Default|GetWidget) true false)))

(event OnComponentEndOverlap(Sphere)
  (params (OverlappedComponent :type Primitive%20Component%20Object%20Reference) (OtherActor :type Actor%20Object%20Reference) (OtherComp :type Primitive%20Component%20Object%20Reference) (OtherBodyIndex :type Integer))
  (Utilities|Casting|CastToBP_FirstPersonCharacter OtherActor)
  (if (Variables|Default|GetCanInteract)
    (Rendering|SetVisibility (Variables|Default|GetWidget) false false)
    (Variables|Default|SetCanRess"E" false)))

(event Custom|CustomEvent
  (params (Can%20Interact :type Boolean))
  (if (Variables|Default|GetCanInteract)
    (if Can%20Interact
      _)))

(event EventPick-upItems
  (bind _asbp_first_person_character (Utilities|Casting|CastToBP_FirstPersonCharacter (Game|GetPlayerCharacter 0)))
  (Variables|/Game/FirstPerson/Blueprints/BP_FirstPersonCharacter.BP_FirstPersonCharacter_C|SetDataCount _asbp_first_person_character (+ 1 (Variables|/Game/FirstPerson/Blueprints/BP_FirstPersonCharacter.BP_FirstPersonCharacter_C|GetDataCount _asbp_first_person_character)))
  (Audio|PlaySound2D "/Game/data_Collection/ytmp3free_cc_data-sound-effect-27-data-research-youtubemp3free_org.ytmp3free_cc_data-sound-effect-27-data-research-youtubemp3free_org" 1.0 1.0 0.0 0 0)
  (Actor|DestroyActor))

(fn ConstructionScript)