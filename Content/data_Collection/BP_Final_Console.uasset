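; BP_Final_Console is the end-of-level console, which checks the player's collected data when Pick-upItems fires.
; An overlap sphere shows or hides a widget for the first-person character while CanInteract is set.
; With a DataCount of at least ten, it plays a sound, adds a fade-to-black widget and restarts the level after a delay.
; Otherwise it only plays a different sound.
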(event OnComponentBeginOverlap(Sphere)
  (params (OverlappedComponent :type Primitive%20Component%20Object%20Reference) (OtherActor :type Actor%20Object%20Reference) (OtherComp :type Primitive%20Component%20Object%20Reference) (OtherBodyIndex :type Integer) (bFromSweep :type Boolean) (SweepResult :type Hit%20Result%20Structure%20%28by%20ref%29))
  (Utilities|Casting|CastToBP_FirstPersonCharacter OtherActor)
  (if (Variables|Default|GetCanInteract)
    (Rendering|SetVisibility (Variables|Default|GetWidget) true false)))

(event OnComponentEndOverlap(Sphere)
  (params (OverlappedComponent :type Primitive%20Component%20Object%20Reference) (OtherActor :type Actor%20Object%20Reference) (OtherComp :type Primitive%20Component%20Object%20Reference) (OtherBodyIndex :type Integer))
  (Utilities|Casting|CastToBP_FirstPersonCharacter OtherActor)
  (if (Variables|Default|GetCanInteract)
    (Rendering|SetVisibility (Variables|Default|GetWidget) false false)
    (Variables|Default|SetCanRess"E" false)))

(event Custom|CustomEvent
  (params (Can%20Interact :type Boolean))
  (if (Variables|Default|GetCanInteract)
    (if Can%20Interact
      _)))

(event EventPick-upItems
  (bind _asbp_first_person_character (Utilities|Casting|CastToBP_FirstPersonCharacter (Game|GetPlayerCharacter 0)))
  (if (>= (Variables|/Game/FirstPerson/Blueprints/BP_FirstPersonCharacter.BP_FirstPersonCharacter_C|GetDataCount _asbp_first_person_character) 10)
    (Audio|PlaySound2D "/Game/data_Collection/ytmp3free_cc_data-sound-effect-27-data-research-youtubemp3free_org.ytmp3free_cc_data-sound-effect-27-data-research-youtubemp3free_org" 1.0 1.0 0.0 0 0)
    (bind _returnvalue (UserInterface|CreateWidget "/Game/data_Collection/Fade_To_Black.Fade_To_Black_C" (Game|GetPlayerController 0)))
    (UserInterface|Viewport|AddtoViewport _returnvalue 0)
    (Utilities|FlowControl|Delay 3.0)
    (Development|ExecuteConsoleCommand "Restartlevel" 0)
    (else
      (Audio|PlaySound2D "/Game/data_Collection/robotv2.robotv2" 1.0 1.0 0.0 0 0))))

(fn ConstructionScript)